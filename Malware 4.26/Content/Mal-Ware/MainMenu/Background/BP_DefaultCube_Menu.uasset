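; BP_DefaultCube_Menu shows the main menu and holds run state for a minigame game: score, lives and timer value.
; BeginPlay creates the menu widget, and SetCamera switches the view to the menu camera.
; RandomMinigame flags either the tank or trolley game, starting BPTank for the former, and shortens CurrentTime at each rising score threshold.
; Death decrements lives or shows the end screen when none remain.
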(event `self.ReceiveBeginPlay`
  (set `self.CurrentTime` (`self.BaseTime`))
  (bind _returnvalue (`|CreateWidget` "/Game/Mal-Ware/MainMenu/Widgets/MainMenu.MainMenu_C"))
  (`UserWidget.AddToViewport` _returnvalue 0))

(event `SetCamera`
  (bind _returnvalue (`GameplayStatics.GetActorOfClass` "/Game/Mal-Ware/MainMenu/Background/BP_CameraMenu.BP_CameraMenu_C"))
  (`PlayerController.SetViewTargetWithBlend` (`GameplayStatics.GetPlayerController` 0) _returnvalue 0.0 "VTBlend_Linear" 0.0 false))

(fn `Death`
  (if (<= (`self.Lives`) 0)
    (bind _returnvalue (`|CreateWidget` "/Game/Mal-Ware/MainMenu/Widgets/EndScreen.EndScreen_C"))
    (`UserWidget.AddToViewport` _returnvalue 0)
    (else
      (bind _output_get (set `self.Lives` (- (`self.Lives`) 1)))
      (`KismetSystemLibrary.PrintString` (`KismetStringLibrary.Conv_IntToString` _output_get)))))

(fn `RandomMinigame`
  (if (>= (`self.GameScore`) (`self.Score*5`))
    (`self.ReduceTime`)
    (`KismetSystemLibrary.PrintString` "Reduced time"))
  (switch `int` (`KismetMathLibrary.RandomInteger` 2)
    (:`0`
      (`KismetSystemLibrary.PrintString` "Tank")
      (set `self.TankGame` true)
      (bind _returnvalue (`GameplayStatics.GetActorOfClass` "/Game/Mal-Ware/Tank/BPTank.BPTank_C"))
      (set `/Game/Mal-Ware/Tank/BPTank.IsStarted?` true _returnvalue))
    (:`1`
      (`KismetSystemLibrary.PrintString` "Trolly")
      (set `self.TrolleyGame` true))))

(fn `ReduceTime`
  (bind _output_get (set `self.CurrentTime` (/ (`self.CurrentTime`) 1.1)))
  (`KismetSystemLibrary.PrintString` (`KismetStringLibrary.Conv_DoubleToString` _output_get))
  (set `self.Score*5` (+ (`self.Score*5`) 5)))

(fn `Score+`
  (set `self.GameScore` (+ (`self.GameScore`) 1)))

(fn `UserConstructionScript`)